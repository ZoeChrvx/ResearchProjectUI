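; BP_Button is a shootable in-world menu button that starts the game, opens the options level or quits.
; It pushes its label into a WBP_TextButton widget component and starts with a fixed hit life.
; Each BP_Bullet hit on the box lowers that life and recolors the text through a color curve.
; At zero the cube hides and the Play, Option or Quit flag selects the action.
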(event OnComponentHit(Box)
  (params (HitComponent :type Primitive%20Component%20Object%20Reference) (OtherActor :type Actor%20Object%20Reference) (OtherComp :type Primitive%20Component%20Object%20Reference) (NormalImpulse :type Vector :default "0, 0, 0") (Hit :type Hit%20Result%20Structure%20%28by%20ref%29))
  (if (== (Utilities|GetClass OtherActor) "/Game/Player/BP_Bullet.BP_Bullet_C")
    (bind _output_get (Variables|Life|SetButtonLife_CurrentValue (- (Variables|Life|GetButtonLife_CurrentValue) 1)))
    (Variables|/Script/UMG.UserWidget|SetColorAndOpacity (Variables|Default|GetRefTextButton) (Math|Curves|GetLinearColorValue (Variables|Life|GetCurveColorText) (Math|Conversions|ToFloat(Integer) _output_get)))
    (if (== (Variables|Life|GetButtonLife_CurrentValue) 0)
      (Rendering|SetVisibility (Variables|Default|GetCube) false false)
      (if (Variables|ButtonType|GetPlay)
        (Game|OpenLevel(byObjectReference) "/Game/Level/L_Game.L_Game")
        (elif (Variables|ButtonType|GetOption)
          (Game|OpenLevel(byObjectReference) "/Game/Level/L_Option.L_Option")
          (elif (Variables|ButtonType|GetQuit)
            (Game|QuitGame 0 "Quit" false)))))))

(event EventBeginPlay
  (bind _aswbp_text_button (Utilities|Casting|CastToWBP_TextButton (UserInterface|GetWidget (Variables|Default|GetWidget))))
  (Variables|Default|SetRefTextButton _aswbp_text_button)
  (Variables|/Game/UI/WBP_TextButton.WBP_TextButton_C|SetButton_Txt _aswbp_text_button (Variables|Life|GetEditButton_Text))
  (bind _output_get (Variables|Life|SetButtonLife_MaxValue 10))
  (bind _output_get_2 (Variables|Life|SetButtonLife_CurrentValue _output_get))
  (Variables|/Script/UMG.UserWidget|SetColorAndOpacity (Variables|Default|GetRefTextButton) (Math|Curves|GetLinearColorValue (Variables|Life|GetCurveColorText) (Math|Conversions|ToFloat(Integer) _output_get_2))))

(fn ConstructionScript)