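; BP_Sign is a sign actor that displays editable text through a WBP_SignText widget.
; On BeginPlay it casts the Widget component's widget to WBP_SignText and caches the reference.
; It copies EditTxtSign into the widget's SigntxtText only when both the Sound and Sensitivity flags are false.
; The construction script is empty and no tick or overlap logic runs.
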(event EventBeginPlay
  (bind _aswbp_sign_text (Utilities|Casting|CastToWBP_SignText (UserInterface|GetWidget (Variables|Default|GetWidget))))
  (bind _output_get (Variables|Default|SetRef%20SignText _aswbp_sign_text))
  (if (== (or (Variables|Default|GetSound) (Variables|Default|GetSensitivity)) false)
    (Variables|/Game/UI/WBP_SignText.WBP_SignText_C|SetSigntxt_Text _output_get (Variables|Default|GetEditTxtSign))))

(event Collision|EventActorBeginOverlap
  (params (OtherActor :type Actor%20Object%20Reference)))

(event EventTick
  (params (DeltaSeconds :type Float%20%28single-precision%29)))

(fn ConstructionScript)