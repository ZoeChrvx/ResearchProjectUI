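; Shootable options button that raises or lowers a sound or sensitivity number shown on a linked sign.
; On BeginPlay it sets its WBP_TextButton label and curve-driven color, then writes the default value to RefSign's text.
; BP_Bullet hits on the Box step the value chosen by boolean flags, clamped, and update the sign.
; Each button stores its own values and only changes displayed text, applying no actual setting.
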(event OnComponentHit(Box)
  (params (HitComponent :type Primitive%20Component%20Object%20Reference) (OtherActor :type Actor%20Object%20Reference) (OtherComp :type Primitive%20Component%20Object%20Reference) (NormalImpulse :type Vector :default "0, 0, 0") (Hit :type Hit%20Result%20Structure%20%28by%20ref%29))
  (if (== (Utilities|GetClass OtherActor) "/Game/Player/BP_Bullet.BP_Bullet_C")
    (if (Variables|ButtonType|GetMoreSensi)
      (Utilities|IsValid (Variables|Default|GetRefSign)
        (:Is%20Valid
          (bind _output_get (Variables|Default|SetSensiValue (Math|Integer|Clamp(Integer) (+ (Variables|Default|GetSensiValue) 1) 0 10)))
          (Variables|/Game/UI/WBP_SignText.WBP_SignText_C|SetSigntxt_Text (Variables|/Game/Blueprint/BP_Sign.BP_Sign_C|GetRef%20SignText (Variables|Default|GetRefSign)) (Utilities|Text|ToText(Integer) _output_get))))
      (elif (Variables|ButtonType|GetLessSensi)
        (Utilities|IsValid (Variables|Default|GetRefSign)
          (:Is%20Valid
            (bind _output_get_2 (Variables|Default|SetSensiValue (Math|Integer|Clamp(Integer) (- (Variables|Default|GetSensiValue) 1) 0 10)))
            (Variables|/Game/UI/WBP_SignText.WBP_SignText_C|SetSigntxt_Text (Variables|/Game/Blueprint/BP_Sign.BP_Sign_C|GetRef%20SignText (Variables|Default|GetRefSign)) (Utilities|Text|ToText(Integer) _output_get_2))))
        (elif (Variables|ButtonType|GetMoreSound)
          (Utilities|IsValid (Variables|Default|GetRefSign)
            (:Is%20Valid
              (bind _output_get_3 (Variables|Default|SetSoundValue (Math|Integer|Clamp(Integer) (+ (Variables|Default|GetSoundValue) 1) 0 10)))
              (Variables|/Game/UI/WBP_SignText.WBP_SignText_C|SetSigntxt_Text (Variables|/Game/Blueprint/BP_Sign.BP_Sign_C|GetRef%20SignText (Variables|Default|GetRefSign)) (Utilities|Text|ToText(Integer) _output_get_3))))
          (elif (Variables|ButtonType|GetLessSound)
            (Utilities|IsValid (Variables|Default|GetRefSign)
              (:Is%20Valid
                (bind _output_get_4 (Variables|Default|SetSoundValue (Math|Integer|Clamp(Integer) (- (Variables|Default|GetSoundValue) 1) 0 10)))
                (Variables|/Game/UI/WBP_SignText.WBP_SignText_C|SetSigntxt_Text (Variables|/Game/Blueprint/BP_Sign.BP_Sign_C|GetRef%20SignText (Variables|Default|GetRefSign)) (Utilities|Text|ToText(Integer) _output_get_4))))))))))

(event EventBeginPlay
  (bind _refsign (Variables|Default|GetRefSign))
  (bind _ref_signtext (Variables|/Game/Blueprint/BP_Sign.BP_Sign_C|GetRef%20SignText _refsign))
  (bind _aswbp_text_button (Utilities|Casting|CastToWBP_TextButton (UserInterface|GetWidget (Variables|Default|GetWidget))))
  (Variables|Default|SetRefTextButton _aswbp_text_button)
  (Variables|/Game/UI/WBP_TextButton.WBP_TextButton_C|SetButton_Txt _aswbp_text_button (Variables|Life|GetEditButton_Text))
  (bind _output_get (Variables|Life|SetButtonLife_MaxValue 10))
  (Variables|/Script/UMG.UserWidget|SetColorAndOpacity (Variables|Default|GetRefTextButton) (Math|Curves|GetLinearColorValue (Variables|Life|GetCurveColorText) (Math|Conversions|ToFloat(Integer) _output_get)))
  (Variables|Default|SetSoundValue 5)
  (Variables|Default|SetSensiValue 5)
  (if (Variables|/Game/Blueprint/BP_Sign.BP_Sign_C|GetSound _refsign)
    (Variables|/Game/UI/WBP_SignText.WBP_SignText_C|SetSigntxt_Text _ref_signtext (Utilities|Text|ToText(Integer) (Variables|Default|GetSoundValue)))
    (elif (Variables|/Game/Blueprint/BP_Sign.BP_Sign_C|GetSensitivity _refsign)
      (Variables|/Game/UI/WBP_SignText.WBP_SignText_C|SetSigntxt_Text _ref_signtext (Utilities|Text|ToText(Integer) (Variables|Default|GetSensiValue))))))

(fn ConstructionScript)